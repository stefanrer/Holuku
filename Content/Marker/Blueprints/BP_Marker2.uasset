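; HUD Blueprint that draws objective markers for distant actors tracked by the World game mode.
; Each DrawHUD pass loops the game mode's Actors array and draws M_ObjectiveMarker for actors at least 30 m from the player.
; Positions are projected to screen, shifted by OffsetPos and clamped to the viewport, with no behind-camera check.
; An unconnected branch that draws text and a marker above on-screen objects never runs.
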(event EventDrawHUD
  (params (SizeX :type Integer) (SizeY :type Integer))
  (bind _returnvalue (Game|GetPlayerController 0))
  (bind _offsetpos (Variables|Default|GetOffsetPos))
  (bind _offsetpos_2 (Variables|Default|GetOffsetPos))
  (bind _returnvalue_2 (/ _offsetpos 2.0))
  (bind _returnvalue_3 (Math|Float|Truncate _offsetpos_2))
  (bind (_sizex _sizey) (HUD|GetViewportSize _returnvalue))
  (bind _asworld (Utilities|Casting|CastToWorld (Game|GetGameMode)))
  (for _array_element (Variables|/Game/Gamemode/World.World_C|GetActors _asworld)
    (if (>= (Math|Vector|Distance(Vector) (Transformation|GetActorLocation (Game|Player|GetPlayerPawn 0)) (Transformation|GetActorLocation _array_element)) 3e+03)
      (Class|HUD|DrawMaterialSimple "/Game/Marker/Material/M_ObjectiveMarker.M_ObjectiveMarker" (Math|Float|Clamp(Float) (+ (.x (.ScreenPosition (Class|GameplayStatics|ProjectWorldtoScreen (Game|GetPlayerController 0) (Transformation|GetActorLocation _array_element) false))) _returnvalue_2) 0.0 (Math|Conversions|ToFloat(Integer) (+ _sizex _returnvalue_3))) (Math|Float|Clamp(Float) (+ (.y (.ScreenPosition (Class|GameplayStatics|ProjectWorldtoScreen (Game|GetPlayerController 0) (Transformation|GetActorLocation _array_element) false))) _returnvalue_2) 0.0 (Math|Conversions|ToFloat(Integer) (+ _sizey _returnvalue_3))) 256.0 256.0 0.175 false))))

(fn ConstructionScript)