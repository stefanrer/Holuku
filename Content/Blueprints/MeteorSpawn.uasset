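; MeteorSpawn fills a region with a field of roughly a thousand Meteor actors on BeginPlay.
; Each spawn location is random within the box whose opposite corners are the world positions of the Sphere and Sphere1 components.
; Rotation is randomized on all axes, and scale is random with extra jitter on Y and Z for irregular shapes.
; Each meteor's Rock component has shadow casting disabled after spawning.
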(event EventBeginPlay
  (bind _returnvalue (Math|Random|RandomFloatinRange 1e+01 5e+01))
  (bind _sphere (Variables|Default|GetSphere))
  (bind _sphere1 (Variables|Default|GetSphere1))
  (bind _returnvalue_2 (Transformation|GetWorldLocation _sphere))
  (bind _returnvalue_3 (Transformation|GetWorldLocation _sphere1))
  (for _index (range 0 1000)
    (bind _returnvalue_4 (Game|SpawnActorfromClass "/Game/Blueprints/Pawn/Rock/Meteor.Meteor_C" (Math|Transform|MakeTransform (Math|Vector|MakeVector (Math|Random|RandomFloatinRange (.x _returnvalue_2) (.x _returnvalue_3)) (Math|Random|RandomFloatinRange (.y _returnvalue_2) (.y _returnvalue_3)) (Math|Random|RandomFloatinRange (.z _returnvalue_2) (.z _returnvalue_3))) (Math|Rotator|MakeRotator (Math|Random|RandomFloatinRange 0.0 359.0) (Math|Random|RandomFloatinRange 0.0 359.0) (Math|Random|RandomFloatinRange 0.0 359.0)) (Math|Vector|MakeVector _returnvalue (+ _returnvalue (Math|Random|RandomFloatinRange 1.0 5.0)) (+ _returnvalue (Math|Random|RandomFloatinRange 1.0 5.0)))) "Undefined" 0 0))
    (Rendering|SetCastShadow (Variables|/Game/Blueprints/Pawn/Rock/Meteor.Meteor_C|GetRock _returnvalue_4) false)))

(fn ConstructionScript)