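; Player spaceship pawn that flies with pitch, yaw and roll, fires twin projectiles and loads the "Tunel" level once defeated enemies exceed nine.
; Thrust interpolates DesiredSpeed, which Move applies each Tick as a swept local offset, snapping CurrentSpeed to it through a zero interp speed.
; Collisions nudge rotation toward the hit normal.
; Shield recharges on Tick unless Hit is set, which clears after a delay; BeginPlay adds the Shield_Hp widget.
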(event Custom|HitDelay
  (Utilities|FlowControl|Delay 1.0)
  (Variables|Default|SetHit false))

(event EventBeginPlay
  (bind _returnvalue (UserInterface|CreateWidget "/Game/Blueprints/Pawn/Widget/Shield_Hp.Shield_Hp_C"))
  (UserInterface|Viewport|AddtoViewport _returnvalue 0))

(event Collision|EventHit
  (params (MyComp :type Primitive%20Component%20Object%20Reference) (Other :type Actor%20Object%20Reference) (OtherComp :type Primitive%20Component%20Object%20Reference) (bSelfMoved :type Boolean) (HitLocation :type Vector :default "0, 0, 0") (HitNormal :type Vector :default "0, 0, 0") (NormalImpulse :type Vector :default "0, 0, 0") (Hit :type Hit%20Result%20Structure%20%28by%20ref%29))
  ;[1 1 1] Deflect when colliding
  (Transformation|SetActorRotation (Math|Rotator|Lerp(Rotator) (Transformation|GetActorRotation) (Math|Conversions|RotationFromXVector HitNormal) 0.03 true)))

(event EventTick
  (params (DeltaSeconds :type Float%20%28single-precision%29))
  (CallFunction|Move)
  (CallFunction|ShieldRec)
  (if (> (Variables|Default|GetDefeated%20Enemyes) 9.0)
    (Game|OpenLevel(byName) "Tunel")))

(event Input|ActionEvents|InputActionExit
  (params (Key :type Key%20Structure :default "None"))
  (:Pressed
    (Game|QuitGame 0 "Quit" false)))

(event Input|AxisEvents|InputAxisRoll
  (params (AxisValue :type Float%20%28single-precision%29))
  ;[1 1 1] Ролы
  (if (!= AxisValue 0.0)
    (Transformation|AddActorLocalRotation (Math|Rotator|MakeRotator AxisValue 0.0 0.0) false false)))

(event Input|AxisEvents|InputAxisThrust
  (params (AxisValue :type Float%20%28single-precision%29))
  ;[1 1 1] Придание ускорения вперед назад
  (if (> AxisValue 0.0)
    (Variables|Default|SetDesiredSpeed (Math|Interpolation|FInterpTo (Variables|Default|GetDesiredSpeed) (Variables|Default|GetMaxSpeed) (Utilities|Time|GetWorldDeltaSeconds) (Variables|Default|GetAccelerat)))
    (elif (< AxisValue 0.0)
      (Variables|Default|SetDesiredSpeed (Math|Interpolation|FInterpTo (Variables|Default|GetDesiredSpeed) (* (/ (Variables|Default|GetMaxSpeed) 2.0) -1.0) (Utilities|Time|GetWorldDeltaSeconds) (Variables|Default|GetAccelerat))))))

(event Input|AxisEvents|InputAxisYaw
  (params (AxisValue :type Float%20%28single-precision%29))
  ;[1 1 1] Поворот экрана с мышкой
  (if (!= AxisValue 0.0)
    (Transformation|AddActorLocalRotation (Math|Rotator|MakeRotator 0.0 0.0 AxisValue) false false)))

(event Input|AxisEvents|InputAxisPitch
  (params (AxisValue :type Float%20%28single-precision%29))
  ;[1 1 1] Поворот экрана с мышкой
  (if (!= AxisValue 0.0)
    (Transformation|AddActorLocalRotation (Math|Rotator|MakeRotator 0.0 AxisValue 0.0) false false)))

(event Input|MouseEvents|LeftMouseButton
  (params (Key :type Key%20Structure :default "None"))
  (bind _returnvalue (Utilities|Time|GetWorldDeltaSeconds))
  (bind _returnvalue_2 (Transformation|GetActorRotation))
  (bind _self self)
  (bind _maxspeed (Variables|Default|GetMaxSpeed))
  (bind _returnvalue_3 (Transformation|GetActorForwardVector _self))
  (bind _returnvalue_4 (Transformation|GetActorLocation _self))
  (bind _returnvalue_5 (Transformation|GetActorRightVector _self))
  (bind _returnvalue_6 (* _maxspeed _returnvalue))
  (bind _returnvalue_7 (* _returnvalue_3 1e+02))
  (bind _returnvalue_8 (+ _returnvalue_6 2e+02))
  (bind _returnvalue_9 (+ _returnvalue_4 _returnvalue_7))
  ;[1 1 1] Стреьба
  (:Pressed
    (Audio|PlaySound2D "/Game/Sound/lasershot_Cue.lasershot_Cue" 1.0 1.0 0.0 0 0)
    (Game|SpawnActorfromClass "/Game/Blueprints/Pawn/WorldProjectile.WorldProjectile_C" (Math|Transform|MakeTransform (+ _returnvalue_9 (* _returnvalue_5 5e+01)) _returnvalue_2 "1,1,1") "Undefined" 0 _returnvalue_8 _returnvalue_3 0)
    (Game|SpawnActorfromClass "/Game/Blueprints/Pawn/WorldProjectile.WorldProjectile_C" (Math|Transform|MakeTransform (+ _returnvalue_9 (* _returnvalue_5 -5e+01)) _returnvalue_2 "1,1,1") "Undefined" 0 _returnvalue_8 _returnvalue_3 0)))

(fn ConstructionScript)

(fn Move
  (bind _output_get (Variables|Default|SetCurrentSpeed (Math|Interpolation|FInterpTo (Variables|Default|GetCurrentSpeed) (Variables|Default|GetDesiredSpeed) (Utilities|Time|GetWorldDeltaSeconds) (/ 0.0 2.0))))
  (Transformation|AddActorLocalOffset (Math|Vector|MakeVector _output_get 0.0 0.0) true false))

(fn ShieldRec
  (if (Variables|Default|GetHit)
    (CallFunction|HitDelay)
    (elif (< (Variables|Default|GetShield) 1e+02)
      (Variables|Default|SetShield (+ (Math|Float|Clamp(Float) (Variables|Default|GetShield) 0.0 1e+02) (* (Utilities|Time|GetWorldDeltaSeconds) (Variables|Default|GetShiledRecoveryEncrement)))))))