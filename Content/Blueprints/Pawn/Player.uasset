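; Player spaceship pawn that flies forward along world X, with boost, steering, roll, twin-projectile fire and a rear-view camera.
; Each tick, four line traces ignoring "Enemy" actors scale side and vertical movement down near surfaces; upward clearance also drives a red screen overlay.
; A blocking hit during forward movement, except on a finish actor, triggers an explosion, increments the saved death count and reloads the level.
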(event Custom|RightTrace
  (bind _returnvalue (Transformation|GetActorLocation))
  ;[1 1 1] RightTrace and Slowing down when to close
  (bind (_outhit _returnvalue_2) (Collision|LineTraceByChannel _returnvalue (+ _returnvalue (* "0,1.000000, 0" 500)) "TraceTypeQuery1" false (Variables|Default|GetIgnore%20Actors) "None"))
  (if _returnvalue_2
    (Variables|Default|SetDistanceScaleRight (/ (- (.Distance (Collision|BreakHitResult _outhit)) 2.5e+02) 2.5e+02))))

(event Custom|DownTrace
  (bind _returnvalue (Transformation|GetActorLocation))
  ;[1 1 1] DownTrace and Slowing down when to close
  (bind (_outhit _returnvalue_2) (Collision|LineTraceByChannel _returnvalue (+ _returnvalue (* "0,0.000000,1.000000" -500)) "TraceTypeQuery1" false (Variables|Default|GetIgnore%20Actors) "None"))
  (if _returnvalue_2
    (Variables|Default|SetDistanceScaleDown (/ (- (.Distance (Collision|BreakHitResult _outhit)) 1e+02) 4e+02))))

(event Custom|LeftTrace
  (bind _returnvalue (Transformation|GetActorLocation))
  ;[1 1 1] LeftTrace and Slowing down when to close
  (bind (_outhit _returnvalue_2) (Collision|LineTraceByChannel _returnvalue (+ _returnvalue (* "0,1.000000, 0" -500)) "TraceTypeQuery1" false (Variables|Default|GetIgnore%20Actors) "None"))
  (if _returnvalue_2
    (Variables|Default|SetDistanceScaleLeft (/ (- (.Distance (Collision|BreakHitResult _outhit)) 2.5e+02) 2.5e+02))))

(event Custom|DIe
  (bind _save_instance (Variables|Default|GetSave%20Instance))
  (Utilities|FlowControl|DoOnce false
    (:Completed
      (Effects|SpawnEmitteratLocation "/Game/ExplosionParticles/Particles/Expl/Explosion.Explosion" (Transformation|GetActorLocation) "0, 0, 0" "10.000000,10.000000,10.000000")
      (Components|DestroyComponent (Variables|Default|GetStaticMesh))
      (Variables|/Game/Blueprints/Pawn/Save.Save_C|SetDeaths _save_instance (+ (Variables|/Game/Blueprints/Pawn/Save.Save_C|GetDeaths _save_instance) 1.0))
      (SaveGame|SaveGametoSlot (Variables|Default|GetSave%20Instance) (Variables|Default|GetSaveSlotName))
      (Utilities|FlowControl|Delay 1.0)
      (bind _returnvalue (Game|GetCurrentLevelName true))
      (Game|OpenLevel(byName) (Utilities|String|StringToName _returnvalue)))))

(event Custom|UpTrace
  (bind _returnvalue (Transformation|GetActorLocation))
  ;[1 1 1] UpTrace and Slowing down when to close
  (bind (_outhit _returnvalue_2) (Collision|LineTraceByChannel _returnvalue (+ _returnvalue (* "0,0.000000,1.000000" 500)) "TraceTypeQuery2" false (Variables|Default|GetIgnore%20Actors) "None"))
  (if _returnvalue_2
    (Variables|Default|SetDistanceScaleUp (/ (- (.Distance (Collision|BreakHitResult _outhit)) 1e+02) 4e+02))))

(event EventBeginPlay
  (bind _outactors (Actor|GetAllActorswithTag "Enemy"))
  (Variables|Default|SetIgnore%20Actors _outactors)
  (bind _returnvalue (SaveGame|LoadGamefromSlot (Variables|Default|GetSaveSlotName)))
  (bind _assave (Utilities|Casting|CastToSave _returnvalue)
    (:then
      (Variables|Default|SetSave%20Instance _assave))
    (:CastFailed
      (bind _returnvalue_2 (SaveGame|CreateSaveGameObject "/Game/Blueprints/Pawn/Save.Save_C"))
      (Variables|Default|SetSave%20Instance _returnvalue_2)))
  (SaveGame|SaveGametoSlot (Variables|Default|GetSave%20Instance) (Variables|Default|GetSaveSlotName))
  (Variables|Default|SetDeaths (Variables|/Game/Blueprints/Pawn/Save.Save_C|GetDeaths (Variables|Default|GetSave%20Instance)))
  (bind _returnvalue_3 (UserInterface|CreateWidget "/Game/Blueprints/Pawn/Widget/RedScreen.RedScreen_C"))
  (UserInterface|Viewport|AddtoViewport _returnvalue_3 0)
  (Variables|Default|SetRedscreen _returnvalue_3))

(event EventTick
  (params (DeltaSeconds :type Float%20%28single-precision%29))
  ;[1 1 1] Handle Tick
  (CallFunction|RightTrace)
  (CallFunction|LeftTrace)
  (CallFunction|UpTrace)
  (CallFunction|DownTrace)
  (bind _spaceshipspeedforward (CallFunction|ShipForwardSpeed))
  (CallFunction|RedScreenOpacity)
  (bind _sweephitresult (Transformation|AddActorWorldOffset (Math|Vector|MakeVector (* _spaceshipspeedforward DeltaSeconds) 0.0 0.0) true))
  (if (.bBlockingHit (Collision|BreakHitResult _sweephitresult))
    (Utilities|Casting|CastTofinish (.HitActor (Collision|BreakHitResult _sweephitresult))
      (:CastFailed
        (CallFunction|DIe)))))

(event Input|ActionEvents|InputActionChangecameratobackview
  (params (Key :type Key%20Structure :default "None"))
  (:Pressed
    (Components|Activation|SetActive (Variables|Default|Getbackview) true false)
    (Components|Activation|SetActive (Variables|Default|GetCamera) false false))
  (:Released
    (Components|Activation|SetActive (Variables|Default|Getbackview) false false)
    (Components|Activation|SetActive (Variables|Default|GetCamera) true false)))

(event Input|ActionEvents|InputActionFire
  (params (Key :type Key%20Structure :default "None"))
  (bind _returnvalue (Utilities|Time|GetWorldDeltaSeconds))
  (bind _self self)
  (bind _spaceshipmaxspeed (Variables|Default|GetSpaceShipMaxSpeed))
  (bind _returnvalue_2 (Transformation|GetActorForwardVector _self))
  (bind _returnvalue_3 (Transformation|GetActorLocation _self))
  (bind _returnvalue_4 (Transformation|GetActorRightVector _self))
  (bind _returnvalue_5 (* _spaceshipmaxspeed _returnvalue))
  (bind _returnvalue_6 (* _returnvalue_2 1e+02))
  (bind _returnvalue_7 (+ _returnvalue_5 2e+02))
  (bind _returnvalue_8 (+ _returnvalue_3 _returnvalue_6))
  ;[1 1 1] Firing
  (:Pressed
    (Audio|PlaySound2D "/Game/Sound/lasershot_Cue.lasershot_Cue" 1.0 1.0 0.0 0 0)
    (Game|SpawnActorfromClass "/Game/Blueprints/Pawn/Projectile.Projectile_C" (Math|Transform|MakeTransform (+ _returnvalue_8 (* _returnvalue_4 5e+01)) "0, 0, 0" "1.500000,1.500000,1.500000") "Undefined" 0 _returnvalue_7 0)
    (Game|SpawnActorfromClass "/Game/Blueprints/Pawn/Projectile.Projectile_C" (Math|Transform|MakeTransform (+ _returnvalue_8 (* _returnvalue_4 -5e+01)) "0, 0, 0" "1.500000,1.500000,1.500000") "Undefined" 0 _returnvalue_7 0)))

(event Input|ActionEvents|InputActionTunnelSpeedBoost
  (params (Key :type Key%20Structure :default "None"))
  (:Pressed
    (Variables|Default|SetSpacePressed true))
  (:Released
    (Variables|Default|SetSpacePressed false)))

(event Input|AxisEvents|InputAxisVerticalmovement
  (params (AxisValue :type Float%20%28single-precision%29))
  (bind _returnvalue (Utilities|Time|GetWorldDeltaSeconds))
  ;[1 1 1] Handle VerticalMovement
  (Math|Float|CompareFloat AxisValue 0.0
    (:>
      (Transformation|AddActorWorldOffset (Math|Vector|MakeVector 0.0 0.0 (* AxisValue 1e+03 (Variables|Default|GetDistanceScaleUp) _returnvalue)) true))
    (:<
      (Transformation|AddActorWorldOffset (Math|Vector|MakeVector 0.0 0.0 (* AxisValue 1e+03 (Variables|Default|GetDistanceScaleDown) _returnvalue)) true))))

(event Input|AxisEvents|InputAxisRoll
  (params (AxisValue :type Float%20%28single-precision%29))
  ;[1 1 1] Handle Roll
  (if (!= AxisValue 0.0)
    (Transformation|AddActorLocalRotation (Math|Rotator|MakeRotator (* AxisValue (Utilities|Time|GetWorldDeltaSeconds) 1e+02) 0.0 0.0) false false)))

(event Input|AxisEvents|InputAxisSidemovement
  (params (AxisValue :type Float%20%28single-precision%29))
  (bind _returnvalue (Utilities|Time|GetWorldDeltaSeconds))
  ;[1 1 1] Handle SideMovement
  (Math|Float|CompareFloat AxisValue 0.0
    (:>
      (Transformation|AddActorWorldOffset (Math|Vector|MakeVector 0.0 (* AxisValue 1.5e+03 (Variables|Default|GetDistanceScaleRight) _returnvalue) 0.0) true))
    (:<
      (Transformation|AddActorWorldOffset (Math|Vector|MakeVector 0.0 (* AxisValue 1.5e+03 (Variables|Default|GetDistanceScaleLeft) _returnvalue) 0.0) true))))

(fn ConstructionScript)

(fn ShipForwardSpeed
  (if (Variables|Default|GetSpacePressed)
    (Variables|Default|SetSpaceShipForwardSpeed (+ (Math|Float|Clamp(Float) (Variables|Default|GetSpaceShipForwardSpeed) (+ 0.0 (* (Variables|Default|GetSpeedStep) (Variables|Default|GetSpeedStepMinX))) (Variables|Default|GetSpaceShipMaxSpeed)) (Variables|Default|GetSpeedStep)))
    (else
      (Variables|Default|SetSpaceShipForwardSpeed (- (Math|Float|Clamp(Float) (Variables|Default|GetSpaceShipForwardSpeed) (+ 0.0 (* (Variables|Default|GetSpeedStep) (Variables|Default|GetSpeedStepMinX))) (Variables|Default|GetSpaceShipMaxSpeed)) (Variables|Default|GetSpeedStep)))))
  (return (Variables|Default|GetSpaceShipForwardSpeed)))

(fn RedScreenOpacity
  (bind _distancescaleup (Variables|Default|GetDistanceScaleUp))
  (bind _redscreen (Variables|Default|GetRedscreen))
  (if (and (<= _distancescaleup 0.5) (> _distancescaleup 0.2))
    (Variables|/Game/Blueprints/Pawn/Widget/RedScreen.RedScreen_C|SetOpac _redscreen 0.3)
    (elif (<= _distancescaleup 0.2)
      (Variables|/Game/Blueprints/Pawn/Widget/RedScreen.RedScreen_C|SetOpac _redscreen 0.6)
      (else
        (Variables|/Game/Blueprints/Pawn/Widget/RedScreen.RedScreen_C|SetOpac _redscreen 0.0)))))