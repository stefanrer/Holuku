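; Projectile actor that flies forward, spawns a hit effect on impact and increments the hit count on any FloatingObject it strikes.
; Each Tick, it line-traces the next step on the Camera channel, ignoring its Instigator, then moves by Speed without sweep or DeltaSeconds scaling.
; A blocking hit spawns the emitter at an X-offset from the impact point and destroys the projectile, which also expires after MaxExistingTime.
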(event EventTick
  (params (DeltaSeconds :type Float%20%28single-precision%29))
  (bind _returnvalue (Transformation|GetActorLocation))
  (bind _returnvalue_2 (Transformation|GetActorForwardVector))
  (bind _speed (Variables|Default|GetSpeed))
  (bind _returnvalue_3 (* _returnvalue_2 _speed))
  (bind _returnvalue_4 (+ _returnvalue _returnvalue_3))
  (bind _outhit (Collision|LineTraceByChannel _returnvalue _returnvalue_4 "TraceTypeQuery2" false (Utilities|Array|MakeArray (Variables|Actor|GetInstigator)) "None"))
  (Transformation|SetActorLocation _returnvalue_4 false false)
  (Variables|Default|Settime (+ (Variables|Default|Gettime) DeltaSeconds))
  (if (> (Variables|Default|Gettime) (Variables|Default|GetMaxExistingTime))
    (Actor|DestroyActor)
    (elif (.bBlockingHit (Collision|BreakHitResult _outhit))
      (Effects|SpawnEmitteratLocation "/Game/ExplosionParticles/Particles/Expl/Hit.Hit" (Math|Vector|MakeVector (- (.X (Math|Vector|BreakVector (.ImpactPoint (Collision|BreakHitResult _outhit)))) 1e+02) (.Y (Math|Vector|BreakVector (.ImpactPoint (Collision|BreakHitResult _outhit)))) (.Z (Math|Vector|BreakVector (.ImpactPoint (Collision|BreakHitResult _outhit))))))
      (bind _asfloating_object (Utilities|Casting|CastToFloatingObject (.HitActor (Collision|BreakHitResult _outhit)))
        (:then
          (Variables|/Game/Blueprints/Pawn/Rock/FloatingObject.FloatingObject_C|Sethits _asfloating_object (+ (Variables|/Game/Blueprints/Pawn/Rock/FloatingObject.FloatingObject_C|Gethits _asfloating_object) 1.0))
          (Actor|DestroyActor))
        (:CastFailed
          (Actor|DestroyActor))))))

(fn ConstructionScript)