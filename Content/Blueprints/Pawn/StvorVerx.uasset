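; StvorVerx is an actor with a Cube component that moves vertically while the player is within range, apparently a sliding upper gate or door leaf.
; Every tick it compares its distance to player pawn 0 against a fixed threshold, playing a timeline inside it and stopping it outside.
; The timeline track, scaled by Naprav, sets the cube's relative Z with sweep; leaving range halts it without reversing.
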(event Custom|Start
  (bind _newtrack_0 (Timeline|Timeline_0 Play)
    (:Update
      (Transformation|SetRelativeLocation (Variables|Default|GetCube) (Math|Vector|MakeVector 0.0 0.0 (* _newtrack_0 (Variables|Default|GetNaprav))) true false))))

(event Custom|Stop
  (bind _newtrack_0 (Timeline|Timeline_0 Stop)
    (:Update
      (Transformation|SetRelativeLocation (Variables|Default|GetCube) (Math|Vector|MakeVector 0.0 0.0 (* _newtrack_0 (Variables|Default|GetNaprav))) true false))))

(event EventTick
  (params (DeltaSeconds :type Float%20%28single-precision%29))
  (bind _returnvalue (Game|Player|GetPlayerPawn 0))
  (Utilities|IsValid _returnvalue
    (:Is%20Valid
      (if (< (Math|Vector|Distance(Vector) (Transformation|GetActorLocation self) (Transformation|GetActorLocation _returnvalue)) 3e+04)
        (CallFunction|Start)
        (else
          (CallFunction|Stop))))))

(fn ConstructionScript)