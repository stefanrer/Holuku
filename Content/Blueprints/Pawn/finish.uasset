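; Finish-line actor that ends the level when the Player pawn overlaps it.
; On overlap it shows the FinishMenu widget, switches to UI-only input and reveals the mouse cursor.
; It then spawns a hugely scaled Explosion emitter at its location, destroys its Cube component and destroys the player.
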(event EventBeginPlay)

(event Collision|EventActorBeginOverlap
  (params (OtherActor :type Actor%20Object%20Reference))
  (bind _returnvalue (Game|GetPlayerController 0))
  (bind _asplayer (Utilities|Casting|CastToPlayer OtherActor))
  (bind _returnvalue_2 (UserInterface|CreateWidget "/Game/Blueprints/Pawn/Widget/FinishMenu.FinishMenu_C"))
  (UserInterface|Viewport|AddtoViewport _returnvalue_2 0)
  (Input|SetInputModeUIOnly _returnvalue _returnvalue_2 "DoNotLock")
  (Variables|/Script/Engine.PlayerController|SetbShowMouseCursor _returnvalue true)
  (Effects|SpawnEmitteratLocation "/Game/ExplosionParticles/Particles/Expl/Explosion.Explosion" (Transformation|GetActorLocation) "0, 0, 0" "100.000000,100.000000,100.000000")
  (Components|DestroyComponent (Variables|Default|GetCube))
  (Actor|DestroyActor _asplayer))

(event EventTick
  (params (DeltaSeconds :type Float%20%28single-precision%29)))

(fn ConstructionScript)