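; StoppinglaserSpawn is a spawner that emits a continuous barrage of StopProjectile actors across the stretch between the player start and the finish.
; BeginPlay caches the PlayerSpawnPoint and Finish actors.
; Every Tick spawns four projectiles, each at a random X between the first of each of those actors, keeping the spawner's own Y and Z.
; The spawn rate has no timer or throttle, so it follows the frame rate.
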(event EventTick
  (params (DeltaSeconds :type Float%20%28single-precision%29))
  (bind _returnvalue (Transformation|GetActorLocation))
  (bind (_x _y _z) (Math|Vector|BreakVector _returnvalue))
  (Game|SpawnActorfromClass "/Game/Blueprints/Pawn/StopProjectile.StopProjectile_C" (Math|Transform|MakeTransform (Math|Vector|MakeVector (Math|Random|RandomFloatinRange (.X (Math|Vector|BreakVector (Transformation|GetActorLocation (Utilities|Array|Get(acopy) (stale EventBeginPlay _outactors_2))))) (.X (Math|Vector|BreakVector (Transformation|GetActorLocation (Utilities|Array|Get(acopy) (stale EventBeginPlay _outactors)))))) _y _z) "0, 0, 0" "1,1,1") "Undefined" 0 0)
  (Game|SpawnActorfromClass "/Game/Blueprints/Pawn/StopProjectile.StopProjectile_C" (Math|Transform|MakeTransform (Math|Vector|MakeVector (Math|Random|RandomFloatinRange (.X (Math|Vector|BreakVector (Transformation|GetActorLocation (Utilities|Array|Get(acopy) (stale EventBeginPlay _outactors_2))))) (.X (Math|Vector|BreakVector (Transformation|GetActorLocation (Utilities|Array|Get(acopy) (stale EventBeginPlay _outactors)))))) _y _z) "0, 0, 0" "1,1,1") "Undefined" 0 0)
  (Game|SpawnActorfromClass "/Game/Blueprints/Pawn/StopProjectile.StopProjectile_C" (Math|Transform|MakeTransform (Math|Vector|MakeVector (Math|Random|RandomFloatinRange (.X (Math|Vector|BreakVector (Transformation|GetActorLocation (Utilities|Array|Get(acopy) (stale EventBeginPlay _outactors_2))))) (.X (Math|Vector|BreakVector (Transformation|GetActorLocation (Utilities|Array|Get(acopy) (stale EventBeginPlay _outactors)))))) _y _z) "0, 0, 0" "1,1,1") "Undefined" 0 0)
  (Game|SpawnActorfromClass "/Game/Blueprints/Pawn/StopProjectile.StopProjectile_C" (Math|Transform|MakeTransform (Math|Vector|MakeVector (Math|Random|RandomFloatinRange (.X (Math|Vector|BreakVector (Transformation|GetActorLocation (Utilities|Array|Get(acopy) (stale EventBeginPlay _outactors_2))))) (.X (Math|Vector|BreakVector (Transformation|GetActorLocation (Utilities|Array|Get(acopy) (stale EventBeginPlay _outactors)))))) _y _z) "0, 0, 0" "1,1,1") "Undefined" 0 0))

(event EventBeginPlay
  (bind _outactors (Actor|GetAllActorsOfClass "/Game/Blueprints/Pawn/finish.finish_C"))
  (bind _outactors_2 (Actor|GetAllActorsOfClass "/Game/Blueprints/PlayerSpawnPoint.PlayerSpawnPoint_C")))

(fn ConstructionScript)