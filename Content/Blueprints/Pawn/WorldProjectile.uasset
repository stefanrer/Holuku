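; WorldProjectile is a projectile that flies along its forward vector and damages Enemy actors.
; Each Tick it line-traces the next step on the Camera channel, ignoring its Instigator, then teleport-free moves by Speed without sweep or delta-time scaling.
; An Enemy hit loses one Hp and destroys the projectile, while other hits let it continue.
; It also destroys itself once its lifetime reaches MaxExistingTime.
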(event EventTick
  (params (DeltaSeconds :type Float%20%28single-precision%29))
  (bind _returnvalue (Transformation|GetActorLocation))
  (bind _forward_vector (Variables|Default|GetForward%20Vector))
  (bind _speed (Variables|Default|GetSpeed))
  (bind _returnvalue_2 (* _forward_vector _speed))
  (bind _returnvalue_3 (+ _returnvalue _returnvalue_2))
  (Variables|Default|SetTime (+ (Variables|Default|GetTime) DeltaSeconds))
  (bind (_outhit _returnvalue_4) (Collision|LineTraceByChannel _returnvalue _returnvalue_3 "TraceTypeQuery2" false (Utilities|Array|MakeArray (Variables|Actor|GetInstigator)) "None"))
  (Transformation|SetActorLocation _returnvalue_3 false false)
  (if (>= (Variables|Default|GetTime) (Variables|Default|GetMaxExistingTime))
    (Actor|DestroyActor)
    (elif _returnvalue_4
      (bind _asenemy (Utilities|Casting|CastToEnemy (.HitActor (Collision|BreakHitResult _outhit))))
      (Variables|/Game/AI/Enemy.Enemy_C|SetHp _asenemy (- (Variables|/Game/AI/Enemy.Enemy_C|GetHp _asenemy) 1.0))
      (Actor|DestroyActor))))

(fn ConstructionScript)