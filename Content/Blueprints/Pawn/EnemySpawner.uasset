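; Enemy spawner actor that periodically spawns enemies at random positions in the level.
; A looping timer started on BeginPlay spawns a double-scale Enemy within configurable X, Y and Z ranges, skipping spawns that would still collide after adjustment.
; After each spawn attempt it casts the player pawn to SpaceShipPlayer and prints its defeated enemy count as debug output.
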(event Custom|Spawn%20Enemy
  (Game|SpawnActorfromClass "/Game/AI/Enemy.Enemy_C" (Math|Transform|MakeTransform (Math|Vector|MakeVector (Math|Random|RandomFloatinRange (Variables|Default|GetXMin) (Variables|Default|GetXMax)) (Math|Random|RandomFloatinRange (Variables|Default|GetYMin) (Variables|Default|GetYMax)) (Math|Random|RandomFloatinRange (Variables|Default|GetZMin) (Variables|Default|GetZMax))) "0, 0, 0" "2.000000,2.000000,2.000000") "AdjustIfPossibleButDontSpawnIfColliding" 0 0)
  (bind _asspace_ship_player (Utilities|Casting|CastToSpaceShipPlayer (Game|Player|GetPlayerPawn 0)))
  (Development|PrintString (Utilities|String|ToString(Float) (Variables|/Game/Blueprints/Pawn/SpaceShipPlayer.SpaceShipPlayer_C|GetDefeated%20Enemyes _asspace_ship_player))))

(event EventBeginPlay
  (Utilities|Time|SetTimerbyEvent (delegate Custom|Spawn%20Enemy) (Variables|Default|GetSpawnDelay) true))

(fn ConstructionScript)