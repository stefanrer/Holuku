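; Stvor is a moving two-part hazard that kills the player and restarts the current level on contact.
; A timeline slides two cubes in opposite directions along local Y with swept moves.
; A blocking hit on a Player destroys it and reopens the level by name.
; Tick runs the timeline only while the player pawn is within a set distance, and stops it when farther away.
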(event Custom|Start
  (bind _moves (Timeline|Timeline_0 Play)
    (:Update
      (bind _sweephitresult (Transformation|SetRelativeLocation (Variables|Default|GetCube1) (Math|Vector|MakeVector 0.0 _moves 0.0) true false))
      (if (.bBlockingHit (Collision|BreakHitResult _sweephitresult))
        (bind _asplayer (Utilities|Casting|CastToPlayer (.HitActor (Collision|BreakHitResult _sweephitresult)))
          (:then
            (Actor|DestroyActor _asplayer)
            (bind _returnvalue (Game|GetCurrentLevelName true))
            (Game|OpenLevel(byName) (Utilities|String|StringToName _returnvalue)))
          (:CastFailed
            _)))
      (bind _sweephitresult_2 (Transformation|SetRelativeLocation (Variables|Default|GetCube) (Math|Vector|MakeVector 0.0 (* _moves -1.0) 0.0) true false))
      (if (.bBlockingHit (Collision|BreakHitResult _sweephitresult_2))
        (bind _asplayer_2 (Utilities|Casting|CastToPlayer (.HitActor (Collision|BreakHitResult _sweephitresult_2))))
        (Actor|DestroyActor _asplayer_2)
        (bind _returnvalue_2 (Game|GetCurrentLevelName true))
        (Game|OpenLevel(byName) (Utilities|String|StringToName _returnvalue_2))))))

(event Custom|Stop
  (bind _moves (Timeline|Timeline_0 Stop)
    (:Update
      (bind _sweephitresult (Transformation|SetRelativeLocation (Variables|Default|GetCube1) (Math|Vector|MakeVector 0.0 _moves 0.0) true false))
      (if (.bBlockingHit (Collision|BreakHitResult _sweephitresult))
        (bind _asplayer (Utilities|Casting|CastToPlayer (.HitActor (Collision|BreakHitResult _sweephitresult)))
          (:then
            (Actor|DestroyActor _asplayer)
            (bind _returnvalue (Game|GetCurrentLevelName true))
            (Game|OpenLevel(byName) (Utilities|String|StringToName _returnvalue)))
          (:CastFailed
            _)))
      (bind _sweephitresult_2 (Transformation|SetRelativeLocation (Variables|Default|GetCube) (Math|Vector|MakeVector 0.0 (* _moves -1.0) 0.0) true false))
      (if (.bBlockingHit (Collision|BreakHitResult _sweephitresult_2))
        (bind _asplayer_2 (Utilities|Casting|CastToPlayer (.HitActor (Collision|BreakHitResult _sweephitresult_2))))
        (Actor|DestroyActor _asplayer_2)
        (bind _returnvalue_2 (Game|GetCurrentLevelName true))
        (Game|OpenLevel(byName) (Utilities|String|StringToName _returnvalue_2))))))

(event EventTick
  (params (DeltaSeconds :type Float%20%28single-precision%29))
  (bind _returnvalue (Game|Player|GetPlayerPawn 0))
  (Utilities|IsValid _returnvalue
    (:Is%20Valid
      (if (< (Math|Vector|Distance(Vector) (Transformation|GetActorLocation self) (Transformation|GetActorLocation _returnvalue)) 3e+04)
        (CallFunction|Start)
        (else
          (CallFunction|Stop))))))

(fn ConstructionScript)